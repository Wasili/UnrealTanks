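; Player-controllable tank Blueprint that wires input to camera aiming, track movement and firing.
; On BeginPlay it passes the Barrel and Turret components to the aiming setup functions.
; Aim axes rotate the camera rig, yaw on AzimuthSpringArm and pitch on AzimuthGimbal, without moving turret or barrel directly.
; Left and right throttle axes drive each track independently, and the Fire action calls Fire, which is defined outside this graph.
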(event `self.ReceiveBeginPlay`
  (`self.SetAimingComponentBarrel` (`self.Barrel`))
  (`self.SetAimingComponentTurret` (`self.Turret`)))

(event `InputAction|Fire`
  (params (Key :type "Key Structure"))
  (:`Pressed`
    (`self.Fire`)))

(event `InputAxis|AimAzimuth`
  (params (AxisValue :type "Float (single-precision)"))
  (`SceneComponent.K2_AddLocalRotation` (`self.AzimuthSpringArm`) (`KismetMathLibrary.MakeRotator` 0.0 0.0 AxisValue) false false))

(event `InputAxis|Aimelevation`
  (params (AxisValue :type "Float (single-precision)"))
  (`SceneComponent.K2_AddLocalRotation` (`self.AzimuthGimbal`) (`KismetMathLibrary.MakeRotator` 0.0 AxisValue) false false))

(event `InputAxis|LeftTrackThrottle`
  (params (AxisValue :type "Float (single-precision)"))
  (`TankTrack.SetThrottle` (`self.LeftTankTrack`) AxisValue))

(event `InputAxis|RightTrackThrottle`
  (params (AxisValue :type "Float (single-precision)"))
  (`TankTrack.SetThrottle` (`self.RightTankTrack`) AxisValue))

(fn `UserConstructionScript`)